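; Level-end trigger actor that unlocks the next level and shows the Game_Paused widget when the player pawn overlaps it.
; It loads or creates Save_Player in slot "1", matches the current level in BP_GameMode_Pawn's LevelsAssetData and adds the next name to NewUnlockedLevels.
; The save after unlocking writes the created-save reference, not the loaded one.
; It shows the mouse cursor, but the SetGamePaused call is unconnected.
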(event EventBeginPlay)

(event Collision|EventActorBeginOverlap
  (params (OtherActor :type Actor%20Object%20Reference))
  (if (== OtherActor (Game|Player|GetPlayerPawn 0))
    (bind _returnvalue (SaveGame|DoesSaveGameExist "1"))
    (if _returnvalue
      (bind _returnvalue_2 (SaveGame|LoadGamefromSlot "1"))
      (bind _assave_player (Utilities|Casting|CastToSave_Player _returnvalue_2))
      (else
        (bind _returnvalue_3 (SaveGame|CreateSaveGameObject "/Game/Save_Player.Save_Player_C"))
        (SaveGame|SaveGametoSlot _returnvalue_3 "1")))
    (bind _outactors (Actor|GetAllActorsOfClass "/Game/Blueprints/Managers/BP_GameMode_Pawn.BP_GameMode_Pawn_C"))
    (for (_array_element _array_index) (Variables|/Game/Blueprints/Managers/BP_GameMode_Pawn.BP_GameMode_Pawn_C|GetLevels_AssetData (Utilities|Array|Get(acopy) _outactors))
      (bind _returnvalue_4 (Game|GetCurrentLevelName true))
      (if (Utilities|Enum|Equal(Enum) (Utilities|GetObjectName (Class|AssetRegistryHelpers|GetAsset _array_element)) _returnvalue_4)
        (Utilities|Array|Add (Variables|/Game/Save_Player.Save_Player_C|GetNewUnlockedLevels _assave_player) (Utilities|GetObjectName (Class|AssetRegistryHelpers|GetAsset (Utilities|Array|Get(acopy) (Variables|/Game/Blueprints/Managers/BP_GameMode_Pawn.BP_GameMode_Pawn_C|GetLevels_AssetData (Utilities|Array|Get(acopy) _outactors)) (+ _array_index 1)))))
        (SaveGame|SaveGametoSlot _returnvalue_3 "1")
        (Development|PrintString (Utilities|String|Append "Unlocked LEvels: " ""))))
    (Development|PrintString "create widget")
    (bind _foundwidgets (Widget|GetAllWidgetsOfClass "/Game/Widgets/Game_Paused.Game_Paused_C" false))
    (Variables|/Script/Engine.PlayerController|SetbShowMouseCursor (Game|GetPlayerController 0) true)
    (UserInterface|Viewport|AddtoViewport (Utilities|Array|Get(acopy) _foundwidgets) 0)))

(event EventTick
  (params (DeltaSeconds :type Float%20%28single-precision%29)))

(fn ConstructionScript)