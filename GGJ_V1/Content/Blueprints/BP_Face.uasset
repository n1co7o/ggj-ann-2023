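; BP_Face is an actor that drives an animated face material according to whether the player is jumping.
; Its construction script creates a dynamic instance of MAT_FACE_Inst on the Re component.
; BeginPlay finds the first BP_PlayerPawn, and Tick polls its IsJumping flag to choose a FacialExpression value.
; That value is written each frame to the "Animation" scalar parameter on Re's materials.
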(event EventBeginPlay
  (bind _outactors (Actor|GetAllActorsOfClass "/Game/Blueprints/BP_PlayerPawn.BP_PlayerPawn_C"))
  (Variables|Default|SetPlayer (Utilities|Array|Get(acopy) _outactors)))

(event Collision|EventActorBeginOverlap
  (params (OtherActor :type Actor%20Object%20Reference)))

(event EventTick
  (params (DeltaSeconds :type Float%20%28single-precision%29))
  (if (Variables|/Game/Blueprints/BP_PlayerPawn.BP_PlayerPawn_C|GetIsJumping (Variables|Default|GetPlayer))
    (Variables|Default|SetFacial%20expression 0.25)
    (else
      (Variables|Default|SetFacial%20expression 0.0)))
  (Rendering|Material|SetScalarParameterValueonMaterials (Variables|Default|Getre) "Animation" (Variables|Default|GetFacial%20expression)))

(fn ConstructionScript
  (bind _returnvalue (Rendering|Material|CreateDynamicMaterialInstance (Variables|Default|Getre) 0 "/Game/Materials/MAT_FACE_Inst.MAT_FACE_Inst" "None" :!class /Script/Engine.PrimitiveComponent))
  (Variables|Default|SetMaterial _returnvalue))