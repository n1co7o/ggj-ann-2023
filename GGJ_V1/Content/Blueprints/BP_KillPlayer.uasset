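; BP_KillPlayer is a trigger actor that interrupts play with the Game_Escape menu when the player's pawn overlaps it.
; On overlap it loads the Save_Player save, or creates and writes one if none exists.
; It then creates the Game_Escape widget, shows the mouse cursor and pauses the game.
; Disconnected leftover logic for unlocking the next level from the game-mode pawn's level list never runs.
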(event EventBeginPlay)

(event Collision|EventActorBeginOverlap
  (params (OtherActor :type Actor%20Object%20Reference))
  (if (== OtherActor (Game|Player|GetPlayerPawn 0))
    (bind _returnvalue (SaveGame|DoesSaveGameExist "1"))
    (if _returnvalue
      (bind _returnvalue_2 (SaveGame|LoadGamefromSlot "1"))
      (bind _assave_player (Utilities|Casting|CastToSave_Player _returnvalue_2))
      (else
        (bind _returnvalue_3 (SaveGame|CreateSaveGameObject "/Game/Save_Player.Save_Player_C"))
        (SaveGame|SaveGametoSlot _returnvalue_3 "1")))
    (bind _returnvalue_4 (UserInterface|CreateWidget "/Game/Widgets/Game_Escape.Game_Escape_C"))
    (Variables|/Script/Engine.PlayerController|SetbShowMouseCursor (Game|GetPlayerController 0) true)
    (UserInterface|Viewport|AddtoViewport _returnvalue_4 0)
    (Game|SetGamePaused true)))

(event EventTick
  (params (DeltaSeconds :type Float%20%28single-precision%29)))

(fn ConstructionScript)