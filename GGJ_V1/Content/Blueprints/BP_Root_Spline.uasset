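; BP_Root_Spline grows a collidable spline trail, apparently a root, behind the player pawn's mesh.
; A looping timer adds a point once the mesh moves KnotGap from the spline's end, held at Y=0 and offset against its facing by bounds and SafeZone.
; Each new point spawns spline mesh components over the latest indices, using spline tangents.
; The OLD graph's timeline-driven end stretching never runs.
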(event Custom|AddKnot
  (bind _spline (Variables|Default|GetSpline))
  (bind _player_mesh (Variables|Default|GetPlayer%20Mesh))
  (bind _spline_2 (Variables|Default|GetSpline))
  (bind _safe_zone (Variables|Default|GetSafe%20Zone))
  (bind _returnvalue (Transformation|GetWorldLocation _player_mesh))
  (bind _boxextent (Collision|GetComponentBounds _player_mesh))
  (bind _returnvalue_2 (Math|Vector|MakeVector _safe_zone 0.0 0.0))
  (bind _returnvalue_3 (Math|Vector|MakeVector 0.0 0.0 _safe_zone))
  (bind _returnvalue_4 (Math|Vector|GetForwardVector _player_mesh))
  (bind _returnvalue_5 (Math|Vector|MakeVector (.x _boxextent) 0.0 0.0))
  (bind _returnvalue_6 (Math|Vector|MakeVector 0.0 0.0 (.z _boxextent)))
  (bind _returnvalue_7 (* _returnvalue_5 _returnvalue_2))
  (bind _returnvalue_8 (* _returnvalue_6 _returnvalue_3))
  (if (>= (Math|Vector|Distance(Vector) _returnvalue (Spline|GetLocationatSplinePoint _spline_2 (Spline|GetNumberOfSplinePoints _spline_2) "World")) (Variables|Default|GetKnotGap))
    (Spline|AddSplinePoint (Variables|Default|GetSpline) (Math|Vector|MakeVector (.x (select (> (.x _returnvalue_4) 0.0) (- _returnvalue _returnvalue_7) (+ _returnvalue _returnvalue_7))) 0.0 (.z (select (> (.z _returnvalue_4) 0.0) (- _returnvalue _returnvalue_8) (+ _returnvalue _returnvalue_8)))) "World" true)
    (for _index (range (- (Spline|GetNumberOfSplinePoints (Variables|Default|GetSpline)) 2) (Spline|GetNumberOfSplinePoints (Variables|Default|GetSpline)))
      (bind _returnvalue_9 (AddComponent|AddSplineMeshComponent false))
      (SplineMesh|SetForwardAxis _returnvalue_9 "Y" true)
      (Collision|SetCollisionEnabled _returnvalue_9 "QueryAndPhysics")
      (SplineMesh|SetStartandEnd _returnvalue_9 (Spline|GetLocationatSplinePoint _spline _index "Local") (Spline|GetTangentatSplinePoint _spline _index "Local") (Spline|GetLocationatSplinePoint _spline (+ _index 1) "Local") (Spline|GetTangentatSplinePoint _spline (+ _index 1) "Local") true :!class /Script/Engine.SplineMeshComponent))))

(event EventTick
  (params (DeltaSeconds :type Float%20%28single-precision%29)))

(event EventBeginPlay
  (bind _outactors (Actor|GetAllActorsOfClass "/Game/Blueprints/BP_PlayerPawn.BP_PlayerPawn_C"))
  (bind _output_get (Variables|Default|SetPlayer_Pawn_Ref (Utilities|Array|Get(acopy) _outactors)))
  (Variables|Default|SetPlayer%20Mesh (Variables|/Game/Blueprints/BP_PlayerPawn.BP_PlayerPawn_C|GetSM_PlayerMesh _output_get))
  (Utilities|Time|SetTimerbyEvent (delegate Custom|AddKnot) (Variables|Default|GetTick) true)
  (Spline|ClearSplinePoints (Variables|Default|GetSpline) true)
  (Spline|AddSplinePoint (Variables|Default|GetSpline) (Transformation|GetWorldLocation (Variables|Default|GetPlayer%20Mesh)) "World" true)
  (if (Variables|Default|GetShow%20Spline)
    (Development|ExecuteConsoleCommand "show splines" 0)))

(fn ConstructionScript)