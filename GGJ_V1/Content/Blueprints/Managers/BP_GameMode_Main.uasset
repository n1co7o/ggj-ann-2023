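; Main game mode that builds the level-finish menu from the main quest levels when play begins.
; It queries the Asset Registry for assets in the MainQuest levels folder, so the list is not hardcoded.
; It creates a Game_Level_Finish widget and fills its vertical box with a button per asset, each labelled and given the asset's name.
; The widget is stored but not added to the viewport here.
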(event EventBeginPlay
  (bind _returnvalue (Class|AssetRegistryHelpers|GetAssetRegistry))
  ;[1 1 1] Populate list of levels
  (Class|AssetRegistry|GetAssetsbyClass :self _returnvalue)
  (bind _outassetdata (Class|AssetRegistry|GetAssetsbyPath _returnvalue "/Game/Levels/MainQuest" false false))
  (Variables|Default|SetMQ_Levels _outassetdata)
  (bind _returnvalue_2 (UserInterface|CreateWidget "/Game/Widgets/Game_Level_Finish.Game_Level_Finish_C"))
  (bind _output_get (Variables|Default|SetLevelFinishWidget _returnvalue_2))
  (for _array_element (Variables|Default|GetMQ_Levels)
    (Development|PrintString (Utilities|GetObjectName (Class|AssetRegistryHelpers|GetAsset _array_element)))
    (bind _returnvalue_3 (UserInterface|CreateWidget "/Game/Widgets/Button.Button_C"))
    (Variables|/Game/Widgets/Button.Button_C|SetText _returnvalue_3 (Utilities|Text|ToText(String) (Utilities|GetObjectName (Class|AssetRegistryHelpers|GetAsset _array_element))))
    (Widget|Panel|AddChild (Variables|/Game/Widgets/Game_Level_Finish.Game_Level_Finish_C|GetVerticalBox_45 _output_get) _returnvalue_3)
    (Default|SetButtonTextEvent _returnvalue_3 (Utilities|String|StringToName (Utilities|GetObjectName (Class|AssetRegistryHelpers|GetAsset _array_element))))))

(event EventTick
  (params (DeltaSeconds :type Float%20%28single-precision%29)))

(fn ConstructionScript)