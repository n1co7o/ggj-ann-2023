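; Game mode Blueprint that builds a level-select list and records the current level as unlocked on BeginPlay.
; Queries the Asset Registry for assets in the MainQuest levels folder, adding a named button for each to a Game_Paused widget stored as LevelFinishWidget.
; Then loads the Save_Player slot, appends the current level name to NewUnlockedLevels and saves it back.
; The widget is never added to the viewport here.
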(event EventBeginPlay
  (bind _returnvalue (Class|AssetRegistryHelpers|GetAssetRegistry))
  (Class|AssetRegistry|GetAssetsbyClass :self _returnvalue)
  (bind _outassetdata (Class|AssetRegistry|GetAssetsbyPath _returnvalue "/Game/Levels/MainQuest" false false))
  (Variables|Default|SetLevels_AssetData _outassetdata)
  (bind _returnvalue_2 (UserInterface|CreateWidget "/Game/Widgets/Game_Paused.Game_Paused_C"))
  (bind _output_get (Variables|Default|SetLevelFinishWidget _returnvalue_2))
  (for _array_element (Variables|Default|GetLevels_AssetData)
    (bind _returnvalue_3 (UserInterface|CreateWidget "/Game/Widgets/Button.Button_C"))
    (Variables|/Game/Widgets/Button.Button_C|SetText _returnvalue_3 (Utilities|Text|ToText(String) (Utilities|GetObjectName (Class|AssetRegistryHelpers|GetAsset _array_element))))
    (Widget|Panel|AddChild (Variables|/Game/Widgets/Game_Paused.Game_Paused_C|GetVerticalBox_45 _output_get) _returnvalue_3)
    (Default|SetButtonTextEvent _returnvalue_3 (Utilities|String|StringToName (Utilities|GetObjectName (Class|AssetRegistryHelpers|GetAsset _array_element)))))
  (bind _returnvalue_4 (SaveGame|LoadGamefromSlot "1"))
  (bind _assave_player (Utilities|Casting|CastToSave_Player _returnvalue_4))
  (bind _returnvalue_5 (Game|GetCurrentLevelName true))
  (Utilities|Array|Add (Variables|/Game/Save_Player.Save_Player_C|GetNewUnlockedLevels _assave_player) _returnvalue_5)
  (SaveGame|SaveGametoSlot _returnvalue_4 "1"))

(event EventTick
  (params (DeltaSeconds :type Float%20%28single-precision%29)))

(fn ConstructionScript)